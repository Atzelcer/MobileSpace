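; BP_Star is a configurable star actor whose look is built from exposed variables in the Construction Script.
; It creates dynamic material instances for the star and surface ray meshes, pushes surface, atmosphere and color parameters, and assigns the lens flare material.
; When AtmosphericPhenomena is on, StarPhenomena scatters rays, ejections, explosions, flares and eruptions as static mesh components along random surface normals, using the bounds radius corrected for actor scale.
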(event `self.ReceiveTick`
  (params (DeltaSeconds :type "Float (single-precision)"))
  (set `self.Delta` DeltaSeconds))

(fn `UserConstructionScript`
  (bind _sm_star (`self.SM_Star`))
  (bind _sm_rays (`self.SM_Rays`))
  (bind _sm_rays_2 (`self.SM_Rays`))
  (`|ExecutionSequence`
    (:`then_0`
      ;[1 1 1] Create Dynamic Material Instances
      (bind _returnvalue (`PrimitiveComponent.CreateDynamicMaterialInstance` _sm_rays_2 0 (`PrimitiveComponent.GetMaterial` _sm_rays_2 0) "None"))
      (set `self.DMI_Rays` _returnvalue)
      (bind _returnvalue_2 (`PrimitiveComponent.CreateDynamicMaterialInstance` _sm_star 0 (`PrimitiveComponent.GetMaterial` _sm_star 0) "None"))
      (set `self.DMI_Star` _returnvalue_2))
    (:`then_1`
      ;[1 1 1] Surface Rays
      (if (`self.Activate Surface Rays`)
        (`SceneComponent.SetVisibility` _sm_rays true false)
        (`MaterialInstanceDynamic.SetScalarParameterValue` (`self.DMI_Rays`) "Increment Factor" (`self.Rays Increment Factor`))
        (`MaterialInstanceDynamic.SetScalarParameterValue` (`self.DMI_Rays`) "Brightness" (`self.Rays Brightness`))
        (`MaterialInstanceDynamic.SetVectorParameterValue` (`self.DMI_Rays`) "Rays Color" (`self.Rays Color`))
        (else
          (`SceneComponent.SetVisibility` _sm_rays false false))))
    (:`then_2`
      ;[1 1 1] Cells
      (`MaterialInstanceDynamic.SetScalarParameterValue` (`self.DMI_Star`) "Large Cells Amount" (`self.Large Cells Amount`))
      (`MaterialInstanceDynamic.SetScalarParameterValue` (`self.DMI_Star`) "Large Cells Brightness" (`self.Large Cells Brightness`))
      (`MaterialInstanceDynamic.SetScalarParameterValue` (`self.DMI_Star`) "Large Cells Distortion 1" (`self.Large Cells Distortion 1`))
      (`MaterialInstanceDynamic.SetScalarParameterValue` (`self.DMI_Star`) "Large Cells Distortion 2" (`self.Large Cells Distortion 2`))
      (`MaterialInstanceDynamic.SetScalarParameterValue` (`self.DMI_Star`) "Large Cells Elevation" (`self.Large Cells Elevation`))
      (`MaterialInstanceDynamic.SetScalarParameterValue` (`self.DMI_Star`) "Small Cells Brightness" (`self.Small Cells Brightness`))
      (`MaterialInstanceDynamic.SetScalarParameterValue` (`self.DMI_Star`) "Small Cells Distortion" (`self.Small Cells Distortion`)))
    (:`then_3`
      ;[1 1 1] Bright Zones
      (`MaterialInstanceDynamic.SetScalarParameterValue` (`self.DMI_Star`) "Bright Zones Amount" (`self.Bright Zones Amount`))
      (`MaterialInstanceDynamic.SetScalarParameterValue` (`self.DMI_Star`) "Bright Zones Distortion" (`self.Bright Zones Distortion`))
      (`MaterialInstanceDynamic.SetScalarParameterValue` (`self.DMI_Star`) "Bright Zones Intensity" (`self.Bright Zones Intensity`))
      (`MaterialInstanceDynamic.SetScalarParameterValue` (`self.DMI_Star`) "Bright Zones Thinness" (`self.Bright Zones Thinness`)))
    (:`then_4`
      ;[1 1 1] Filaments and Flares
      (`MaterialInstanceDynamic.SetScalarParameterValue` (`self.DMI_Star`) "Dark Filaments Contrast" (`self.Dark Filaments Contrast`))
      (`MaterialInstanceDynamic.SetScalarParameterValue` (`self.DMI_Star`) "Dark Filaments Coverage" (`self.Dark Filaments Coverage`))
      (`MaterialInstanceDynamic.SetScalarParameterValue` (`self.DMI_Star`) "Flares Brightness" (`self.Flares Brightness`))
      (`MaterialInstanceDynamic.SetScalarParameterValue` (`self.DMI_Star`) "Flares Coverage" (`self.Flares Coverage`))
      (`MaterialInstanceDynamic.SetScalarParameterValue` (`self.DMI_Star`) "Flares Amount" (`self.Flares Amount`))
      (`MaterialInstanceDynamic.SetScalarParameterValue` (`self.DMI_Star`) "Filaments Amount" (`self.Filaments Amount`))
      (`MaterialInstanceDynamic.SetScalarParameterValue` (`self.DMI_Star`) "Filaments Position" (`self.Filaments Position`)))
    (:`then_5`
      ;[1 1 1] Cracks
      (`MaterialInstanceDynamic.SetScalarParameterValue` (`self.DMI_Star`) "Cracks Brightness" (`self.Cracks Brightness`))
      (`MaterialInstanceDynamic.SetScalarParameterValue` (`self.DMI_Star`) "Cracks Distortion" (`self.Cracks Distortion`))
      (`MaterialInstanceDynamic.SetScalarParameterValue` (`self.DMI_Star`) "Cracks Intensity" (`self.Cracks Intensity`))
      (`MaterialInstanceDynamic.SetScalarParameterValue` (`self.DMI_Star`) "Cracks Size" (`self.Cracks Size`))
      (`MaterialInstanceDynamic.SetScalarParameterValue` (`self.DMI_Star`) "Deep Cracks Brightness" (`self.Deep Cracks Brightness`))
      (`MaterialInstanceDynamic.SetScalarParameterValue` (`self.DMI_Star`) "Plates Coverage" (`self.Plates Coverage`)))
    (:`then_6`
      ;[1 1 1] Atmosphere
      (`MaterialInstanceDynamic.SetScalarParameterValue` (`self.DMI_Star`) "Atmosphere Edge" (`self.Atmosphere Edge`))
      (`MaterialInstanceDynamic.SetScalarParameterValue` (`self.DMI_Star`) "Atmosphere Intensity" (`self.Atmosphere Intensity`))
      (`MaterialInstanceDynamic.SetScalarParameterValue` (`self.DMI_Star`) "Haze Edge" (`self.Haze Edge`))
      (`MaterialInstanceDynamic.SetScalarParameterValue` (`self.DMI_Star`) "Haze Intensity" (`self.Haze Intensity`)))
    (:`then_7`
      ;[1 1 1] Global
      (`MaterialInstanceDynamic.SetScalarParameterValue` (`self.DMI_Star`) "Global Brightness" (`self.Global Brightness`))
      (`MaterialInstanceDynamic.SetScalarParameterValue` (`self.DMI_Star`) "Turbolence Speed" (`self.Turbolence Speed`))
      (`MaterialInstanceDynamic.SetScalarParameterValue` (`self.DMI_Star`) "Distortion 2" (`self.Distortion 1`))
      (`MaterialInstanceDynamic.SetScalarParameterValue` (`self.DMI_Star`) "Distortion 3" (`self.Distortion 2`))
      (if (`self.Raise Luminosity with Distance`)
        (`MaterialInstanceDynamic.SetScalarParameterValue` (`self.DMI_Star`) "Luminosity By Distance" 1.0)
        (else
          (`MaterialInstanceDynamic.SetScalarParameterValue` (`self.DMI_Star`) "Luminosity By Distance" 0.0))))
    (:`then_8`
      ;[1 1 1] Colors
      (`MaterialInstanceDynamic.SetVectorParameterValue` (`self.DMI_Star`) "Atmosphere Color" (`self.Atmosphere Color`))
      (`MaterialInstanceDynamic.SetVectorParameterValue` (`self.DMI_Star`) "Color Dark Filaments" (`self.Dark Filaments Color`))
      (`MaterialInstanceDynamic.SetVectorParameterValue` (`self.DMI_Star`) "Color Flares" (`self.Flares Color`))
      (`MaterialInstanceDynamic.SetVectorParameterValue` (`self.DMI_Star`) "Main Color High" (`self.High Zones Color`))
      (`MaterialInstanceDynamic.SetVectorParameterValue` (`self.DMI_Star`) "Main Color Low" (`self.Low Zones Color`))
      (`MaterialInstanceDynamic.SetVectorParameterValue` (`self.DMI_Star`) "Small Cells Color" (`self.Small Cells Color`))
      (`MaterialInstanceDynamic.SetVectorParameterValue` (`self.DMI_Star`) "Small Cells Color" (`self.Small Cells Color`)))
    (:`then_9`
      ;[1 1 1] Star Phenomena
      (if (`self.Atmospheric Phenomena`)
        (`self.Star Phenomena`)))
    (:`then_10`
      (`PrimitiveComponent.SetMaterial` (`self.LensFlare`) 0 (`self.Lensflare Material`)))))