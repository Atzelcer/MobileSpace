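; Example shuriken turret that fires BP_Projectile_Shuriken while the player character is inside its trigger box.
; On Tick, with the character's TrackingMode on, the Middle (yaw) and Top (pitch) parts smoothly aim at the character's TargetPoint; otherwise they ease back to neutral.
; Projectiles spawn from the Arrow through a Delay set by the character's FireRate.
; BeginPlay also fills a description panel widget naming the example's assets.
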(event `self.ReceiveBeginPlay`
  (bind _descriptionpanelwidget (`self.DescriptionPanelWidget`))
  ;[1 1 1] Description Widget
  (bind _returnvalue (`|CreateWidget` "/Game/TurretVFX/BP/Widget/WBP_DescriptionPanel.WBP_DescriptionPanel_C"))
  (bind _output_get (set `self.DescriptionPanelWidget` _returnvalue))
  (`WidgetComponent.SetWidget` (`self.DescriptionWidget`) _output_get)
  (`TextBlock.SetText` (`/Game/TurretVFX/BP/Widget/WBP_DescriptionPanel.TitleText` _descriptionpanelwidget) (`KismetTextLibrary.Conv_StringToText` "Shuriken"))
  (`TextBlock.SetText` (`/Game/TurretVFX/BP/Widget/WBP_DescriptionPanel.DescriptionText` _descriptionpanelwidget) (`KismetTextLibrary.Conv_StringToText` (`KismetStringLibrary.Concat_StrStr` "1) Example Blueprint : BP_Shuriken" " \n" "2) Projectile Particle : P_Shuriken" " \n" "3) Projectile Blueprint : BP_Projectile_Shuriken")))
  (set `self.ProjectileActor` "/Game/TurretVFX/BP/Projectile/BP_Projectile_Shuriken.BP_Projectile_Shuriken_C"))

(event `self.ReceiveTick`
  (params (DeltaSeconds :type "Float (single-precision)"))
  (bind (_relativerotation_roll _relativerotation_pitch _relativerotation_yaw) (`KismetMathLibrary.BreakRotator` (`SceneComponent.RelativeRotation` (`self.Middle`))))
  (bind (_relativerotation_roll_2 _relativerotation_pitch_2) (`KismetMathLibrary.BreakRotator` (`SceneComponent.RelativeRotation` (`self.Top`))))
  (bind (_relativerotation_roll_3 _relativerotation_pitch_3 _relativerotation_yaw_2) (`KismetMathLibrary.BreakRotator` (`SceneComponent.RelativeRotation` (`self.Middle`))))
  (bind (_relativerotation_roll_4 _relativerotation_pitch_4) (`KismetMathLibrary.BreakRotator` (`SceneComponent.RelativeRotation` (`self.Top`))))
  (bind (_returnvalue_roll _returnvalue_pitch _returnvalue_yaw) (`KismetMathLibrary.BreakRotator` (`KismetMathLibrary.RInterpTo` (`KismetMathLibrary.MakeRotator` 0.0 _relativerotation_pitch_2 _relativerotation_yaw) (`KismetMathLibrary.MakeRotator` 0.0 (`self.Pitch`) (`self.Yaw`)) (`self.Delta`) 6.0)))
  (bind (_returnvalue_roll_2 _returnvalue_pitch_2 _returnvalue_yaw_2) (`KismetMathLibrary.BreakRotator` (`KismetMathLibrary.RInterpTo` (`KismetMathLibrary.MakeRotator` 0.0 _relativerotation_pitch_4 _relativerotation_yaw_2) (struct) (`self.Delta`) 6.0)))
  ;[1 1 1] Movement Animation(Stationary Weapon) and Spawning Projectile
  (set `self.Delta` DeltaSeconds)
  (bind _asbp_character (cast `/Game/TurretVFX/BP/BP_Character` (`GameplayStatics.GetPlayerCharacter` 0)))
  (set `self.FireRate` (`/Game/TurretVFX/BP/BP_Character.FireRate` _asbp_character))
  (if (`self.Overlap`)
    (if (`/Game/TurretVFX/BP/BP_Character.TrackingMode` _asbp_character)
      ;;[1 1 1] In the Overlap Area
      (`|ExecutionSequence`
        (:`then_0`
          (bind _asbp_character_2 (cast `/Game/TurretVFX/BP/BP_Character` (`GameplayStatics.GetPlayerCharacter` 0)))
          (bind (_returnvalue_roll_3 _returnvalue_pitch_3 _returnvalue_yaw_3) (`KismetMathLibrary.BreakRotator` (`KismetMathLibrary.FindLookAtRotation` (`SceneComponent.K2_GetComponentLocation` (`self.Arrow`)) (`SceneComponent.K2_GetComponentLocation` (`/Game/TurretVFX/BP/BP_Character.TargetPoint` _asbp_character_2)))))
          (set `self.Yaw` _returnvalue_yaw_3)
          (set `self.Pitch` _returnvalue_pitch_3)
          (`SceneComponent.K2_SetRelativeRotation` (`self.Middle`) (`KismetMathLibrary.MakeRotator` 0.0 0.0 _returnvalue_yaw) false false)
          (`SceneComponent.K2_SetRelativeRotation` (`self.Top`) (`KismetMathLibrary.MakeRotator` 0.0 _returnvalue_pitch) false false))
        (:`then_1`
          ;;;[1 1 1] Fire projectile at character position
          (`KismetSystemLibrary.Delay` (`self.FireRate`))
          (`|SpawnActorFromClass` (`self.ProjectileActor`) (`SceneComponent.K2_GetComponentToWorld` (`self.Arrow`)) "Undefined" "OverrideRootScale" null null)))
      (else
        ;;[1 1 1] Outside the Overlap Area
        (`|ExecutionSequence`
          (:`then_0`
            (cast `/Game/TurretVFX/BP/BP_Character` (`GameplayStatics.GetPlayerCharacter` 0))
            (`|ExecutionSequence`
              (:`then_0`
                (`SceneComponent.K2_SetRelativeRotation` (`self.Middle`) (`KismetMathLibrary.MakeRotator` 0.0 0.0 _returnvalue_yaw_2) false false)
                (`SceneComponent.K2_SetRelativeRotation` (`self.Top`) (`KismetMathLibrary.MakeRotator` 0.0 _returnvalue_pitch_2) false false))))
          (:`then_1`
            ;;;[1 1 1] Spawning Projectile head-on
            (`KismetSystemLibrary.Delay` (`self.FireRate`))
            (`|SpawnActorFromClass` (`self.ProjectileActor`) (`SceneComponent.K2_GetComponentToWorld` (`self.Arrow`)) "Undefined" "OverrideRootScale" null null)))))))

(event `self.Box.OnComponentBeginOverlap`
  (params (OverlappedComponent :type "PrimitiveComponent Object Reference") (OtherActor :type "Actor Object Reference") (OtherComp :type "PrimitiveComponent Object Reference") (OtherBodyIndex :type Integer) (bFromSweep :type Boolean) (SweepResult :type "HitResult Structure (by ref)"))
  ;[1 1 1] Tracking Your Character with Stationary Weapon When Overlapping Capsule Component
  (bind _asbp_character (cast `/Game/TurretVFX/BP/BP_Character` OtherActor))
  (`/Engine/EditorBlueprintResources/StandardMacros.IsValid` _asbp_character
    (:`Is Valid`
      (set `self.Overlap` true))))

(event `self.Box.OnComponentEndOverlap`
  (params (OverlappedComponent :type "PrimitiveComponent Object Reference") (OtherActor :type "Actor Object Reference") (OtherComp :type "PrimitiveComponent Object Reference") (OtherBodyIndex :type Integer))
  ;[1 1 1] Tracking Your Character with Stationary Weapon When Overlapping Capsule Component
  (bind _asbp_character (cast `/Game/TurretVFX/BP/BP_Character` OtherActor))
  (`/Engine/EditorBlueprintResources/StandardMacros.IsValid` _asbp_character
    (:`Is Valid`
      (set `self.Overlap` false))))

(fn `UserConstructionScript`)