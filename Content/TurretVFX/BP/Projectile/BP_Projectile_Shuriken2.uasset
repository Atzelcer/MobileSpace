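; Shuriken projectile Blueprint for the TurretVFX content, flying via a projectile movement component.
; On construction it reads Speed from the first BP_Character in the level to set its initial speed and a proportionally higher max speed.
; On hit it spawns an impact emitter at the hit point, oriented to its sphere.
; It also destroys its trail particle component, then destroys itself after a short delay.
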(event `self.ReceiveHit`
  (params (MyComp :type "PrimitiveComponent Object Reference") (Other :type "Actor Object Reference") (OtherComp :type "PrimitiveComponent Object Reference") (bSelfMoved :type Boolean) (HitLocation :type "Vector Structure") (HitNormal :type "Vector Structure") (NormalImpulse :type "Vector Structure") (Hit :type "HitResult Structure (by ref)"))
  (bind _projectile_particlesystem (`self.Projectile_ParticleSystem`))
  ;[1 1 1] Projectile Hit Event
  (`|ExecutionSequence`
    (:`then_0`
      (`/Engine/EditorBlueprintResources/StandardMacros.IsValid` _projectile_particlesystem
        (:`Is Valid`
          (`ActorComponent.K2_DestroyComponent` _projectile_particlesystem))
        (:`Is Not Valid`
          _))
      (`KismetSystemLibrary.Delay` 0.2)
      (`self.K2_DestroyActor`))
    (:`then_1`
      (`GameplayStatics.SpawnEmitterAtLocation` "/Game/TurretVFX/Sources/Particle/Hit/P_Shuriken2_Hit.P_Shuriken2_Hit" (`.ImpactPoint` (`GameplayStatics.BreakHitResult` Hit)) (`SceneComponent.K2_GetComponentRotation` (`self.Sphere`))))))

(fn `GetDisplayName`)

(fn `UserConstructionScript`
  (bind _projectilemovement (`self.ProjectileMovement`))
  ;[1 1 1] Set Projectile Speed
  (bind _outactors (`GameplayStatics.GetAllActorsOfClass` "/Game/TurretVFX/BP/BP_Character.BP_Character_C"))
  (bind _speed (`/Game/TurretVFX/BP/BP_Character.Speed` (`|GetArrayItem` _outactors)))
  (set `ProjectileMovementComponent.InitialSpeed` _speed _projectilemovement)
  (set `ProjectileMovementComponent.MaxSpeed` (* _speed 1.5) _projectilemovement))